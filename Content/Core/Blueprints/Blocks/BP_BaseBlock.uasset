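; Base brick for a ball-and-block game that tracks HP, shows it by colour and can drop a bonus when destroyed.
; Hits from BP_Ball and BP_ExtraBall lower HP by different amounts, while BP_FakeBall raises it up to a cap.
; SetColour tints a dynamic material instance for certain HP values only, leaving others unchanged.
; At zero HP the block destroys itself and runs chained weighted rolls, spawning at most one bonus actor.
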(event Collision|EventHit
  (params (MyComp :type Primitive%20Component%20Object%20Reference) (Other :type Actor%20Object%20Reference) (OtherComp :type Primitive%20Component%20Object%20Reference) (bSelfMoved :type Boolean) (HitLocation :type Vector :default "0, 0, 0") (HitNormal :type Vector :default "0, 0, 0") (NormalImpulse :type Vector :default "0, 0, 0") (Hit :type Hit%20Result%20Structure%20%28by%20ref%29))
  (Utilities|Casting|CastToBP_Ball Other
    (:then
      (bind _output_get (Variables|Default|SetHP (- (Variables|Default|GetHP) 1)))
      (if (<= _output_get 0) :!label _label
        (Variables|Default|SetSpawnLocationBonus (Transformation|GetWorldLocation (Variables|Default|GetCube)))
        (Actor|DestroyActor)
        (if (Math|Random|RandomBoolwithWeight (Variables|Default|GetSettingDefaultSpeedChanse))
          (Game|SpawnActorfromClass "/Game/Core/Blueprints/Bonuses/Positive/BP_SettingDefaultSpeed.BP_SettingDefaultSpeed_C" (Math|Transform|MakeTransform (Variables|Default|GetSpawnLocationBonus) "0, 0, 0" (Variables|Default|GetSpawn%20Transform%20Scale)) "AlwaysSpawn" 0 0)
          (elif (Math|Random|RandomBoolwithWeight (Variables|Default|GetExtraBallChanse))
            (Game|SpawnActorfromClass "/Game/Core/Blueprints/Bonuses/Positive/BP_AddExtraBallBonus.BP_AddExtraBallBonus_C" (Math|Transform|MakeTransform (Variables|Default|GetSpawnLocationBonus) "0, 0, 0" (Variables|Default|GetSpawn%20Transform%20Scale)) "AlwaysSpawn" 0 0)
            (elif (Math|Random|RandomBoolwithWeight (Variables|Default|GetFakeBallChanse))
              (Game|SpawnActorfromClass "/Game/Core/Blueprints/Bonuses/Negative/BP_AddFakeBonus.BP_AddFakeBonus_C" (Math|Transform|MakeTransform (Variables|Default|GetSpawnLocationBonus) "0, 0, 0" (Variables|Default|GetSpawn%20Transform%20Scale)) "AlwaysSpawn" 0 0)
              (elif (Math|Random|RandomBoolwithWeight (Variables|Default|GetSpeedBallUpChanse))
                (Game|SpawnActorfromClass "/Game/Core/Blueprints/Bonuses/Negative/BP_SpeedBallUp.BP_SpeedBallUp_C" (Math|Transform|MakeTransform (Variables|Default|GetSpawnLocationBonus) "0, 0, 0" (Variables|Default|GetSpawn%20Transform%20Scale)) "AlwaysSpawn" 0 0)))))
        (else
          (CallFunction|SetColour (Variables|Default|GetHP)))))
    (:CastFailed
      (Utilities|Casting|CastToBP_ExtraBall Other
        (:then
          (Variables|Default|SetHP (- (Variables|Default|GetHP) 3))
          (goto _label))
        (:CastFailed
          (Utilities|Casting|CastToBP_FakeBall Other)
          (if (< (+ (Variables|Default|GetHP) 1) 10)
            (Variables|Default|SetHP (+ (Variables|Default|GetHP) 1))
            (goto _label)))))))

(event EventBeginPlay
  (bind _returnvalue (Rendering|Material|CreateDynamicMaterialInstance (Variables|Default|GetCube) 0 0 "None" :!class /Script/Engine.PrimitiveComponent))
  (Variables|Default|SetBlockMaterialInstance _returnvalue)
  (CallFunction|SetColour (Variables|Default|GetHP)))

(fn ConstructionScript)

(fn SetColour
  (params (Lives :type Integer))
  (switch int Lives
    (:1
      (bind _output_get (Variables|Default|SetColorMaterialInstance "(R=0.000000,G=1.000000,B=0.000000,A=1.000000)"))
      (Rendering|Material|SetVectorParameterValue (Variables|Default|GetBlockMaterialInstance) (Variables|Default|GetParameterMaterialInstance) _output_get :!class /Script/Engine.MaterialInstanceDynamic))
    (:2
      (bind _output_get_2 (Variables|Default|SetColorMaterialInstance "(R=1.000000,G=1.000000,B=0.000000,A=1.000000)"))
      (Rendering|Material|SetVectorParameterValue (Variables|Default|GetBlockMaterialInstance) (Variables|Default|GetParameterMaterialInstance) _output_get_2 :!class /Script/Engine.MaterialInstanceDynamic))
    (:3
      (bind _output_get_3 (Variables|Default|SetColorMaterialInstance "(R=0.000000,G=0.000000,B=1.000000,A=1.000000)"))
      (Rendering|Material|SetVectorParameterValue (Variables|Default|GetBlockMaterialInstance) (Variables|Default|GetParameterMaterialInstance) _output_get_3 :!class /Script/Engine.MaterialInstanceDynamic))
    (:4
      (bind _output_get_4 (Variables|Default|SetColorMaterialInstance "(R=1.000000,G=0.000000,B=0.000000,A=1.000000)"))
      (Rendering|Material|SetVectorParameterValue (Variables|Default|GetBlockMaterialInstance) (Variables|Default|GetParameterMaterialInstance) _output_get_4 :!class /Script/Engine.MaterialInstanceDynamic))
    (:5
      (bind _output_get_5 (Variables|Default|SetColorMaterialInstance "(R=0.345602,G=0.000000,B=0.404167,A=1.000000)"))
      (Rendering|Material|SetVectorParameterValue (Variables|Default|GetBlockMaterialInstance) (Variables|Default|GetParameterMaterialInstance) _output_get_5 :!class /Script/Engine.MaterialInstanceDynamic))
    (:8
      (bind _output_get_6 (Variables|Default|SetColorMaterialInstance "(R=0.266667,G=0.186607,B=0.016667,A=1.000000)"))
      (Rendering|Material|SetVectorParameterValue (Variables|Default|GetBlockMaterialInstance) (Variables|Default|GetParameterMaterialInstance) _output_get_6 :!class /Script/Engine.MaterialInstanceDynamic)))
  (return))