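; BP_ExtraBall is an extra ball actor that bounces around the level and has a limited number of lives.
; Each tick it moves along Navigation scaled by Speed with a swept offset, and on a blocking hit reflects its direction from the surface normal's X and Y.
; Hitting a BP_BaseBlock costs it one life, destroying it at zero, and overlapping a KillZVolume destroys it immediately.
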(event Collision|EventActorBeginOverlap
  (params (OtherActor :type Actor%20Object%20Reference))
  (Utilities|Casting|CastToKillZVolume OtherActor)
  (Actor|DestroyActor))

(event EventTick
  (params (DeltaSeconds :type Float%20%28single-precision%29))
  (bind _sweephitresult (Transformation|AddActorWorldOffset (* (* (Variables|Default|GetNavigation) (Variables|Default|GetSpeed)) DeltaSeconds) true))
  (if (.bBlockingHit (Collision|BreakHitResult _sweephitresult))
    (Variables|Default|SetNavigation (Math|Vector|GetReflectionVector (Variables|Default|GetNavigation) (Math|Vector|MakeVector (.x (.Normal (Collision|BreakHitResult _sweephitresult))) (.y (.Normal (Collision|BreakHitResult _sweephitresult))) 0.0)))))

(event Collision|EventHit
  (params (MyComp :type Primitive%20Component%20Object%20Reference) (Other :type Actor%20Object%20Reference) (OtherComp :type Primitive%20Component%20Object%20Reference) (bSelfMoved :type Boolean) (HitLocation :type Vector :default "0, 0, 0") (HitNormal :type Vector :default "0, 0, 0") (NormalImpulse :type Vector :default "0, 0, 0") (Hit :type Hit%20Result%20Structure%20%28by%20ref%29))
  (Utilities|Casting|CastToBP_BaseBlock Other)
  (bind _output_get (Variables|Default|SetExtraBallLives (- (Variables|Default|GetExtraBallLives) 1)))
  (if (== _output_get 0)
    (Actor|DestroyActor)))

(fn ConstructionScript)