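; BP_Test is a functional test that checks where the ball dies relative to the player's carriage.
; PrepareTest casts the player pawn to BP_Carrige, stores its cube's world location and binds to the ball's OnDead event.
; On death, the test fails if the stored carriage Y exceeds the ball's Y, and succeeds otherwise.
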(event Custom|OnDead
  (if (> (.y (Variables|Default|GetCarriage)) (.y (Transformation|GetWorldLocation (Variables|/Game/Core/Blueprints/BP_Ball.BP_Ball_C|GetBall (Variables|/Game/Core/Blueprints/BP_Carrige.BP_Carrige_C|GetBall (stale EventPrepareTest _asbp_carrige))))))
    (Class|FunctionalTest|FinishTest "Failed")
    (else
      (Class|FunctionalTest|FinishTest "Succeeded"))))

(event EventPrepareTest
  (bind _asbp_carrige (Utilities|Casting|CastToBP_Carrige (Game|Player|GetPlayerPawn 0)))
  (Variables|Default|SetCarriage (Transformation|GetWorldLocation (Variables|/Game/Core/Blueprints/BP_Carrige.BP_Carrige_C|GetCube _asbp_carrige)))
  (EventDispatchers|BindEventtoOnDead (Variables|/Game/Core/Blueprints/BP_Carrige.BP_Carrige_C|GetBall _asbp_carrige) (delegate Custom|OnDead)))

(fn ConstructionScript)