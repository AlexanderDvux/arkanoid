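; BP_BaseBonus is a base bonus actor that travels through the level until it touches a KillZVolume or a BP_Carriage.
; On BeginPlay it creates a dynamic material instance on its Cube and tints it with the bonus colour.
; Tick moves it along Navigation at Speed with a frame-rate independent, swept offset.
; Overlapping either target only destroys it; no bonus effect is applied here.
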(event EventBeginPlay
  (bind _returnvalue (Rendering|Material|CreateDynamicMaterialInstance (Variables|Default|GetCube) 0 0 "None" :!class /Script/Engine.PrimitiveComponent))
  (bind _output_get (Variables|Default|SetBonusMaterialInstance _returnvalue))
  (Rendering|Material|SetVectorParameterValue _output_get (Variables|Default|GetBonusParameterName) (Variables|Default|GetBonusColour) :!class /Script/Engine.MaterialInstanceDynamic))

(event Collision|EventActorBeginOverlap
  (params (OtherActor :type Actor%20Object%20Reference))
  (Utilities|Casting|CastToKillZVolume OtherActor
    (:then
      _)
    (:CastFailed
      (Utilities|Casting|CastToBP_Carriage OtherActor)))
  (Actor|DestroyActor))

(event EventTick
  (params (DeltaSeconds :type Float%20%28single-precision%29))
  (Transformation|AddActorWorldOffset (* (* (Variables|Default|GetNavigation) (Variables|Default|GetSpeed)) DeltaSeconds) true))

(fn ConstructionScript)