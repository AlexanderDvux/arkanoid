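; BP_SpeedBallUp is a negative bonus that speeds up the ball when the carriage touches it.
; On actor overlap it runs the parent overlap logic, casts the other actor to BP_Carriage and adds a fixed increment to that carriage's Ball Speed.
; The construction script only calls its parent, and BeginPlay and Tick are disabled.
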(event EventBeginPlay
  (|CallParentFunction) ; This node is disabled and will not be called.\nDrag off pins to build functionality.
)

(event Collision|EventActorBeginOverlap
  (params (OtherActor :type Actor%20Object%20Reference))
  (|CallParentFunction OtherActor)
  (bind _asbp_carriage (Utilities|Casting|CastToBP_Carriage OtherActor))
  (Variables|/Game/Core/Blueprints/BP_Ball.BP_Ball_C|SetSpeed (Variables|/Game/Core/Blueprints/BP_Carriage.BP_Carriage_C|GetBall _asbp_carriage) (+ (Variables|/Game/Core/Blueprints/BP_Ball.BP_Ball_C|GetSpeed (Variables|/Game/Core/Blueprints/BP_Carriage.BP_Carriage_C|GetBall _asbp_carriage)) 1.5)))

(event EventTick
  (params (DeltaSeconds :type Float%20%28single-precision%29))
  (|CallParentFunction DeltaSeconds) ; This node is disabled and will not be called.\nDrag off pins to build functionality.
)

(fn ConstructionScript
  (|CallParentFunction))