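; Player-controlled carriage, apparently the paddle of a ball game, that moves sideways and spawns balls from its capsule.
; The Right axis applies a fixed, swept X offset each update, independent of axis magnitude and frame time.
; BeginPlay calls SpawnBall, which, while lives remain, spawns a ball, binds its OnDead event, decrements and prints BallLives.
; Separate functions spawn extra and fake balls without using lives.
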(event EventBeginPlay
  (CallFunction|SpawnBall))

(event Input|AxisEvents|InputAxisRight
  (params (AxisValue :type Float%20%28single-precision%29))
  (if (> AxisValue 0.0)
    (Transformation|AddActorWorldOffset "-30.000000,0.000000, 0" true)))

(event Input|AxisEvents|InputAxisRight
  (params (AxisValue :type Float%20%28single-precision%29))
  (if (< AxisValue 0.0)
    (Transformation|AddActorWorldOffset "30.000000,-0.000000, 0" true)))

(fn ConstructionScript)

(fn SpawnBall
  (if (> (Variables|Default|GetBallLives) 0)
    (bind _returnvalue (Game|SpawnActorfromClass "/Game/Core/Blueprints/BP_Ball.BP_Ball_C" (Math|Transform|MakeTransform (Transformation|GetWorldLocation (Variables|Default|GetCapsule)) "0, 0, 0" "0.500000,0.500000,0.500000") "AlwaysSpawn" 0 0))
    (bind _output_get (Variables|Default|SetBall _returnvalue))
    (EventDispatchers|BindEventtoOnDead _output_get (EventDispatchers|CreateEvent :!event SpawnBall))
    (bind _result (Math|Integer|DecrementInt (Variables|Default|GetBallLives))
      (:%20%20
        (Development|PrintString (Utilities|String|ToString(Integer) _result) true true "(R=0.154167,G=0.027710,B=0.000000,A=1.000000)" 1e+01)
        (return)))))

(fn SpawnExtraBall
  (bind _returnvalue (Game|SpawnActorfromClass "/Game/Core/Blueprints/BP_ExtraBall.BP_ExtraBall_C" (Math|Transform|MakeTransform (Transformation|GetWorldLocation (Variables|Default|GetCapsule)) "0, 0, 0" "0.500000,0.500000,0.500000") "AlwaysSpawn" 0 0))
  (Variables|Default|SetExtraBAll _returnvalue)
  (return))

(fn SpawnFakeBall
  (bind _returnvalue (Game|SpawnActorfromClass "/Game/Core/Blueprints/BP_FakeBall.BP_FakeBall_C" (Math|Transform|MakeTransform (Transformation|GetWorldLocation (Variables|Default|GetCapsule)) "0, 0, 0" "0.500000,0.500000,0.500000") "AlwaysSpawn" 0 0))
  (Variables|Default|SetFakeBall _returnvalue)
  (return))